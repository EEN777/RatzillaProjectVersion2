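; BP_MinusScoreBase is a breakable score-penalty actor that deducts points from a RatCharacter that overlaps it.
; Its GeometryCollectionComponent is deactivated at BeginPlay and activated on any overlap, which also disables the actor's collision before the character cast.
; For a RatCharacter it then lowers Score, prints the total out of 200 and destroys itself after a short delay.
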(event EventBeginPlay
  (Components|Activation|SetActive (Variables|Default|GetGeometryCollectionComponent) false false))

(event Collision|EventActorBeginOverlap
  (params (OtherActor :type Actor%20Object%20Reference))
  (Components|Activation|SetActive (Variables|Default|GetGeometryCollectionComponent) true false)
  (Collision|SetActorEnableCollision false)
  (bind _asrat_character (Utilities|Casting|CastToRatCharacter OtherActor))
  (bind _output_get (Variables|/Game/ThirdPersonBP/Blueprints/RatCharacter.RatCharacter_C|SetScore _asrat_character (- (Variables|/Game/ThirdPersonBP/Blueprints/RatCharacter.RatCharacter_C|GetScore _asrat_character) 25.0)))
  (Development|PrintString (Utilities|String|Append (Utilities|String|ToString(Float) _output_get) "/200"))
  (Utilities|FlowControl|Delay 2.0)
  (Actor|DestroyActor))

(fn ConstructionScript)