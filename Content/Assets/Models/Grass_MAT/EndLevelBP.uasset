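; EndLevelBP is the level-end trigger that decides whether the player wins or loses.
; On actor overlap it casts the other actor to RatCharacter and sets its EndLevel flag.
; It then pauses the game and opens WinScreen if the rat's Score reaches the 500-point threshold, or LoseScreen otherwise.
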(event EventBeginPlay)

(event Collision|EventActorBeginOverlap
  (params (OtherActor :type Actor%20Object%20Reference))
  (Development|PrintString "Collided")
  (bind _asrat_character (Utilities|Casting|CastToRatCharacter OtherActor))
  (bind _output_get (Variables|/Game/ThirdPersonBP/Blueprints/RatCharacter.RatCharacter_C|SetEndLevel _asrat_character true))
  (if _output_get
    (if (>= (Variables|/Game/ThirdPersonBP/Blueprints/RatCharacter.RatCharacter_C|GetScore _asrat_character) 5e+02)
      (Game|SetGamePaused true)
      (Game|OpenLevel(byName) "WinScreen")
      (else
        (Game|SetGamePaused true)
        (Game|OpenLevel(byName) "LoseScreen")))))

(event EventTick
  (params (DeltaSeconds :type Float%20%28single-precision%29)))

(fn ConstructionScript)